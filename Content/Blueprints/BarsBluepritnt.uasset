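; Bars Blueprint that animates three cubes along their Z scale in sequence, starting one second after BeginPlay.
; Three timelines run in a chain, each starting half a second after the previous one finishes.
; Each timeline update feeds its track value, times a larger multiplier for each successive cube, into AddLocalTransform as a Z scale delta, so scaling is applied incrementally rather than set absolutely.
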(event `self.ReceiveBeginPlay`
  (`KismetSystemLibrary.Delay` 1.0)
  (bind (_direction _newtrack_0) (`Timeline|Timeline_0` :!via `PlayFromStart`)
    (:`Update`
      (`SceneComponent.K2_AddLocalTransform` (`self.Cube`) (`KismetMathLibrary.MakeTransform` (0.0 0.0 0.0) (struct) (`KismetMathLibrary.MakeVector` 1.0 1.0 (* _newtrack_0 1.0))) false false))
    (:`Finished`
      (`KismetSystemLibrary.Delay` 0.5)
      (bind (_direction_2 _newtrack_0_2) (`Timeline|Timeline_1` :!via `PlayFromStart`)
        (:`Update`
          (`SceneComponent.K2_AddLocalTransform` (`self.Cube1`) (`KismetMathLibrary.MakeTransform` (0.0 0.0 0.0) (struct) (`KismetMathLibrary.MakeVector` 1.0 1.0 (* _newtrack_0_2 1.5))) false false))
        (:`Finished`
          (`KismetSystemLibrary.Delay` 0.5)
          (bind (_direction_3 _newtrack_0_3) (`Timeline|Timeline_2` :!via `PlayFromStart`)
            (:`Update`
              (`SceneComponent.K2_AddLocalTransform` (`self.Cube2`) (`KismetMathLibrary.MakeTransform` (0.0 0.0 0.0) (struct) (`KismetMathLibrary.MakeVector` 1.0 1.0 (* _newtrack_0_3 2.0))) false false))))))))

(fn `UserConstructionScript`)